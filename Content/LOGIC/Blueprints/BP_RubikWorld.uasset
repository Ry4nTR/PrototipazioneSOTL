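; Rubik-style world actor that, on pressing E, rolls the sky sphere and two cube components by 90 degrees.
; It caches start and target rotations in parallel arrays, then chains three timelines: an opening shake of the root, a lerped rotation and a closing shake.
; It also sets WorldRotationAxis on the third-person character as the sequence starts and zeroes it during the closing shake.
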(event `self.ReceiveBeginPlay`
  (`self.EnableInput` (`GameplayStatics.GetPlayerController` 0)))

(event `Key|E`
  (params (Key :type "Key Structure"))
  (:`Pressed`
    (`self.SetWorldRotationAxis` (0.0 -1.0 0.0))
    (`self.ArrayCleaning`)
    (`self.AssigningRotationTargets`)
    (bind (_direction _shakeoffset) (`Timeline|TL_ShakeWorldRotationStarted` :!via `PlayFromStart`)
      (:`Update`
        (`SceneComponent.K2_SetRelativeRotation` (`self.DefaultSceneRoot`) (`KismetMathLibrary.MakeRotator` 0.0 _shakeoffset _shakeoffset) false false))
      (:`Finished`
        (`KismetSystemLibrary.Delay` 0.1)
        (bind (_direction_2 _rotation) (`Timeline|TL_RotateRight` :!via `PlayFromStart`)
          (:`Update`
            (`self.RotationOfEachComponent` _rotation))
          (:`Finished`
            (bind (_direction_3 _shakeoffset_2) (`Timeline|TL_ShakeWorldRotationEnded` :!via `PlayFromStart`)
              (:`Update`
                (`SceneComponent.K2_SetRelativeRotation` (`self.DefaultSceneRoot`) (`KismetMathLibrary.MakeRotator` 0.0 _shakeoffset_2 _shakeoffset_2) false false)
                (`self.ResetWorldRotationAxis`)))))))))

(fn `AddRotationTarget`
  (params (AngleDelta :type "Float (double-precision)") (TargetComponent :type "SceneComponent Object Reference"))
  (bind _returnvalue (`SceneComponent.K2_GetComponentRotation` TargetComponent))
  (`KismetArrayLibrary.Array_Add` (`self.ComponentsToRotate`) TargetComponent)
  (`KismetArrayLibrary.Array_Add` (`self.StartRotations`) _returnvalue)
  (`KismetArrayLibrary.Array_Add` (`self.TargetRotations`) (`KismetMathLibrary.MakeRotator` (+ AngleDelta (.roll _returnvalue)) (.pitch _returnvalue) (.yaw _returnvalue))))

(fn `ArrayCleaning`
  (`KismetArrayLibrary.Array_Clear` (`self.ComponentsToRotate`))
  (`KismetArrayLibrary.Array_Clear` (`self.TargetRotations`))
  (`KismetArrayLibrary.Array_Clear` (`self.StartRotations`)))

(fn `AssigningRotationTargets`
  (`self.AddRotationTarget` 90.0 (`Actor.RootComponent` (`self.SkySphereActor`)))
  (`self.AddRotationTarget` 90.0 (`self.CubeRight`))
  (`self.AddRotationTarget` 90.0 (`self.CubeLeft`)))

(fn `ResetWorldRotationAxis`
  (bind _asbp_third_person_character (cast `/Game/LOGIC/Blueprints/BP_ThirdPersonCharacter` (`GameplayStatics.GetPlayerCharacter` 0)))
  (set `/Game/LOGIC/Blueprints/BP_ThirdPersonCharacter.WorldRotationAxis` (0.0 0.0 0.0) _asbp_third_person_character))

(fn `RotateComponent `
  (params (AngleDelta :type "Float (double-precision)") (TargetComponent :type "SceneComponent Object Reference")))

(fn `RotationOfEachComponent`
  (params (InputPin :type "Float (single-precision)"))
  (for (_array_element _array_index) (`self.ComponentsToRotate`)
    (`SceneComponent.K2_SetWorldRotation` _array_element (`KismetMathLibrary.RLerp` (`|GetArrayItem` (`self.StartRotations`) _array_index) (`|GetArrayItem` (`self.TargetRotations`) _array_index) InputPin) false false)))

(fn `SetWorldRotationAxis`
  (params (WorldRotationAxis :type "Vector Structure"))
  (bind _asbp_third_person_character (cast `/Game/LOGIC/Blueprints/BP_ThirdPersonCharacter` (`GameplayStatics.GetPlayerCharacter` 0)))
  (set `/Game/LOGIC/Blueprints/BP_ThirdPersonCharacter.WorldRotationAxis` WorldRotationAxis _asbp_third_person_character))

(fn `UserConstructionScript`)