(fn `Create`
  (locals (X :type Byte) (Y :type Byte) (Z :type Byte))
  (`self.Delete`)
  (for _index (range (`KismetMathLibrary.Conv_ByteToInt` (`self.Depth`)))
    (set `local.X` (`KismetMathLibrary.Conv_IntToByte` _index))
    (for _index_2 (range (`KismetMathLibrary.Conv_ByteToInt` (`self.Width`)))
      (set `local.Y` (`KismetMathLibrary.Conv_IntToByte` _index_2))
      (for _index_3 (range (`KismetMathLibrary.Conv_ByteToInt` (`self.Height`)))
        (set `local.Z` (`KismetMathLibrary.Conv_IntToByte` _index_3))
        (bind _returnvalue (`AddComponent|NODE_AddChildActorComponent-1`))
        (bind _asbp_grid_node (cast `/Game/LOGIC/Blueprints/BP_GridNode` (`ChildActorComponent.ChildActor` _returnvalue)))
        (`self.K2_SetActorRelativeLocation` _asbp_grid_node (* (`KismetMathLibrary.MakeVector` (`KismetMathLibrary.Conv_ByteToDouble` (`local.X`)) (`KismetMathLibrary.Conv_ByteToDouble` (`local.Y`)) (`KismetMathLibrary.Conv_ByteToDouble` (`local.Z`))) (100.0 100.0 100.0)) false false)
        (`BlueprintMapLibrary.Map_Add` (`self.Nodes`) (make `/Game/LOGIC/Structures/F_Byte3` (`local.X`) (`local.Y`) (`local.Z`)) _asbp_grid_node)))))

(fn `Delete`
  (bind (_keypin _valuepin) (`|MapForEach` (`self.Nodes`))
    (:`then`
      (`self.K2_DestroyActor` _valuepin))
    (:`CompletedPin`
      (`BlueprintMapLibrary.Map_Clear` (`self.Nodes`)))))

(fn `GetTopSurface`)

(fn `RemoveTopSurface`)

(fn `UserConstructionScript`)