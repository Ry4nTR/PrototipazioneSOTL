(fn `AddNode`
  (params (GridNode :type "/Game/LOGIC/Blueprints/NICK/BP_GridNode Object Reference") (ToGridPosition :type "/Game/LOGIC/Structures/F_Byte3 Structure"))
  (if (`self.IsGridPositionTakenMacro` ToGridPosition)
    (`KismetSystemLibrary.RaiseScriptError` "ToGridPosition is already taken")
    (else
      (`BlueprintMapLibrary.Map_Add` (`self.Nodes`) ToGridPosition GridNode))))

(fn `Create`
  (locals (X :type Byte) (Y :type Byte) (Z :type Byte))
  (`self.Delete`)
  (for _index (range (`KismetMathLibrary.Conv_ByteToInt` (`self.Depth`)))
    (set `local.X` (`KismetMathLibrary.Conv_IntToByte` _index))
    (for _index_2 (range (`KismetMathLibrary.Conv_ByteToInt` (`self.Width`)))
      (set `local.Y` (`KismetMathLibrary.Conv_IntToByte` _index_2))
      (for _index_3 (range (`KismetMathLibrary.Conv_ByteToInt` (`self.Height`)))
        (set `local.Z` (`KismetMathLibrary.Conv_IntToByte` _index_3))
        (`self.CreateNodeOrHoleAt` (make `/Game/LOGIC/Structures/F_Byte3` (`local.X`) (`local.Y`) (`local.Z`)))))))

(fn `CreateHoleAt`
  (params (GridPosition :type "/Game/LOGIC/Structures/F_Byte3 Structure"))
  (`KismetArrayLibrary.Array_Add` (`self.Holes`) GridPosition))

(fn `CreateNodeAt`
  (params (GridPosition :type "/Game/LOGIC/Structures/F_Byte3 Structure"))
  (bind _returnvalue (`|SpawnActorFromClass` "/Game/LOGIC/Blueprints/NICK/BP_GridNode.BP_GridNode_C" (`self.GetTransform`) "Undefined" "MultiplyWithRoot" null null))
  (`self.K2_AttachToActor` _returnvalue self "None" "KeepRelative" "KeepRelative" "KeepRelative" true)
  (`self.K2_SetActorRelativeLocation` _returnvalue (`self.GetLocalOffsetFromCenterMacro` GridPosition) false true)
  (`self.SetActorRelativeScale3D` _returnvalue (`KismetMathLibrary.Conv_DoubleToVector` (`self.NodeDimension`)))
  (`BlueprintMapLibrary.Map_Add` (`self.Nodes`) GridPosition _returnvalue))

(fn `CreateNodeOrHoleAt`
  (params (GridPosition :type "/Game/LOGIC/Structures/F_Byte3 Structure"))
  (returns (NodeCreated :type Boolean))
  (bind _nodechosen (`self.ShouldGenerateNode`))
  (if _nodechosen
    (`self.CreateNodeAt` GridPosition)
    (else
      (`self.CreateHoleAt` GridPosition)))
  (return _nodechosen))

(fn `Delete`
  (bind (_keypin _valuepin) (`|MapForEach` (`self.Nodes`))
    (:`then`
      (`self.K2_DestroyActor` _valuepin))
    (:`CompletedPin`
      (`BlueprintMapLibrary.Map_Clear` (`self.Nodes`))
      (`KismetArrayLibrary.Array_Clear` (`self.Holes`)))))

(fn `GetLastX`
  (returns (LastX :type Byte))
  (return (- (`self.Depth`) 1)))

(fn `GetLastY`
  (returns (LastY :type Byte))
  (return (- (`self.Width`) 1)))

(fn `GetLastZ`
  (returns (LastZ :type Byte))
  (return (- (`self.Height`) 1)))

(fn `GetLocalBackSurface`
  (returns (LocalBack :type "Map of /Game/LOGIC/Structures/F_Byte3 Structure to /Game/LOGIC/Blueprints/NICK/BP_GridNode Object Reference"))
  (bind _localforwardfacinglayer (`self.GetLocalForwardFacingLayer` 0))
  (return _localforwardfacinglayer))

(fn `GetLocalBottomSurface`
  (returns (LocalBottom :type "Map of /Game/LOGIC/Structures/F_Byte3 Structure to /Game/LOGIC/Blueprints/NICK/BP_GridNode Object Reference"))
  (bind _localupwardfacinglayer (`self.GetLocalUpwardFacingLayer` 0))
  (return _localupwardfacinglayer))

(fn `GetLocalForwardFacingLayer`
  (params (LayerX :type Byte))
  (returns (LocalForwardFacingLayer :type "Map of /Game/LOGIC/Structures/F_Byte3 Structure to /Game/LOGIC/Blueprints/NICK/BP_GridNode Object Reference"))
  (locals (X :type Byte) (Y :type Byte) (Z :type Byte :default 0) (Layer :type "Map of /Game/LOGIC/Structures/F_Byte3 Structure to /Game/LOGIC/Blueprints/NICK/BP_GridNode Object Reference"))
  (set `local.X` LayerX)
  (bind (_layeraxisi _layeraxisj) (`self.IterateOverLayerPositions` (`self.Width`) (`self.Height`))
    (:`LoopBody`
      (set `local.Y` _layeraxisi)
      (set `local.Z` _layeraxisj)
      (`self.AddNodeAtGridPositionInto` (make `/Game/LOGIC/Structures/F_Byte3` (`local.X`) (`local.Y`) (`local.Z`)) (`local.Layer`)))
    (:`Completed`
      (return (`local.Layer`)))))

(fn `GetLocalFrontSurface`
  (returns (LocalFront :type "Map of /Game/LOGIC/Structures/F_Byte3 Structure to /Game/LOGIC/Blueprints/NICK/BP_GridNode Object Reference"))
  (bind _localforwardfacinglayer (`self.GetLocalForwardFacingLayer` (`self.GetLastX`)))
  (return _localforwardfacinglayer))

(fn `GetLocalLayerFacingAxis`
  (params (AxisIndex :type Byte) (OnDepth :type Byte))
  (returns (LayerFacingAxisOnDepth :type "Map of /Game/LOGIC/Structures/F_Byte3 Structure to /Game/LOGIC/Blueprints/NICK/BP_GridNode Object Reference"))
  (locals (Layer :type "Map of /Game/LOGIC/Structures/F_Byte3 Structure to /Game/LOGIC/Blueprints/NICK/BP_GridNode Object Reference"))
  (switch `int` (`KismetMathLibrary.Conv_ByteToInt` AxisIndex)
    (:`Default`
      (`KismetSystemLibrary.RaiseScriptError` "AxisIndex must be either 0, 1 or 2"))
    (:`0`
      (bind _localforwardfacinglayer (`self.GetLocalForwardFacingLayer` OnDepth))
      (set `local.Layer` _localforwardfacinglayer)
      (return (`local.Layer`)))
    (:`1`
      (bind _localrightfacinglayer (`self.GetLocalRightFacingLayer` OnDepth))
      (set `local.Layer` _localrightfacinglayer)
      (return (`local.Layer`)))
    (:`2`
      (bind _localupwardfacinglayer (`self.GetLocalUpwardFacingLayer` OnDepth))
      (set `local.Layer` _localupwardfacinglayer)
      (return (`local.Layer`)))))

(fn `GetLocalLeftSurface`
  (returns (LocalLeft :type "Map of /Game/LOGIC/Structures/F_Byte3 Structure to /Game/LOGIC/Blueprints/NICK/BP_GridNode Object Reference"))
  (bind _localrightfacinglayer (`self.GetLocalRightFacingLayer` 0))
  (return _localrightfacinglayer))

(fn `GetLocalOffsetFromCenter`
  (params (GridPosition :type "/Game/LOGIC/Structures/F_Byte3 Structure"))
  (returns (GridOffset :type "Vector Structure"))
  (return (`self.GetLocalOffsetFromCenterMacro` GridPosition)))

(fn `GetLocalRightFacingLayer`
  (params (LayerY :type Byte))
  (returns (LocalRightFacingLayer :type "Map of /Game/LOGIC/Structures/F_Byte3 Structure to /Game/LOGIC/Blueprints/NICK/BP_GridNode Object Reference"))
  (locals (X :type Byte) (Y :type Byte) (Z :type Byte :default 0) (Layer :type "Map of /Game/LOGIC/Structures/F_Byte3 Structure to /Game/LOGIC/Blueprints/NICK/BP_GridNode Object Reference"))
  (set `local.Y` LayerY)
  (bind (_layeraxisi _layeraxisj) (`self.IterateOverLayerPositions` (`self.Depth`) (`self.Height`))
    (:`LoopBody`
      (set `local.X` _layeraxisi)
      (set `local.Z` _layeraxisj)
      (`self.AddNodeAtGridPositionInto` (make `/Game/LOGIC/Structures/F_Byte3` (`local.X`) (`local.Y`) (`local.Z`)) (`local.Layer`)))
    (:`Completed`
      (return (`local.Layer`)))))

(fn `GetLocalRightSurface`
  (returns (LocalRight :type "Map of /Game/LOGIC/Structures/F_Byte3 Structure to /Game/LOGIC/Blueprints/NICK/BP_GridNode Object Reference"))
  (bind _localrightfacinglayer (`self.GetLocalRightFacingLayer` (`self.GetLastY`)))
  (return _localrightfacinglayer))

(fn `GetLocalTopSurface`
  (returns (LocalTop :type "Map of /Game/LOGIC/Structures/F_Byte3 Structure to /Game/LOGIC/Blueprints/NICK/BP_GridNode Object Reference"))
  (bind _localupwardfacinglayer (`self.GetLocalUpwardFacingLayer` (`self.GetLastZ`)))
  (return _localupwardfacinglayer))

(fn `GetLocalUpwardFacingLayer`
  (params (LayerZ :type Byte))
  (returns (LocalUpwardFacingLayer :type "Map of /Game/LOGIC/Structures/F_Byte3 Structure to /Game/LOGIC/Blueprints/NICK/BP_GridNode Object Reference"))
  (locals (X :type Byte) (Y :type Byte) (Z :type Byte :default 0) (Layer :type "Map of /Game/LOGIC/Structures/F_Byte3 Structure to /Game/LOGIC/Blueprints/NICK/BP_GridNode Object Reference"))
  (set `local.Z` LayerZ)
  (bind (_layeraxisi _layeraxisj) (`self.IterateOverLayerPositions` (`self.Depth`) (`self.Width`))
    (:`LoopBody`
      (set `local.X` _layeraxisi)
      (set `local.Y` _layeraxisj)
      (`self.AddNodeAtGridPositionInto` (make `/Game/LOGIC/Structures/F_Byte3` (`local.X`) (`local.Y`) (`local.Z`)) (`local.Layer`)))
    (:`Completed`
      (return (`local.Layer`)))))

(fn `GetTopSurface`
  (returns (TopSurface :type "Map of /Game/LOGIC/Structures/F_Byte3 Structure to /Game/LOGIC/Blueprints/NICK/BP_GridNode Object Reference"))
  (locals (ForwardDot :type "Float (double-precision)") (RightDot :type "Float (double-precision)") (RightAligned :type Boolean) (UpDot :type "Float (double-precision)") (UpAligned :type Boolean))
  (bind _returnvalue (`KismetMathLibrary.Vector_Up`))
  (bind _returnvalue_2 (`KismetMathLibrary.Dot_VectorVector` (`self.GetActorUpVector`) _returnvalue))
  (bind _returnvalue_3 (`KismetMathLibrary.Dot_VectorVector` (`self.GetActorForwardVector`) _returnvalue))
  (bind _returnvalue_4 (`KismetMathLibrary.Dot_VectorVector` (`self.GetActorRightVector`) _returnvalue))
  (bind _returnvalue_5 (`KismetMathLibrary.Abs` _returnvalue_2))
  (bind _returnvalue_6 (`KismetMathLibrary.Abs` _returnvalue_3))
  (bind _returnvalue_7 (`KismetMathLibrary.Abs` _returnvalue_4))
  (set `local.ForwardDot` _returnvalue_3)
  (set `local.RightDot` _returnvalue_4)
  (set `local.UpDot` _returnvalue_2)
  (if (and (> _returnvalue_6 _returnvalue_7) (> _returnvalue_6 _returnvalue_5))
    (if (> (`local.ForwardDot`) 0.0)
      (bind _localfront (`self.GetLocalFrontSurface`))
      (return _localfront)
      (else
        (bind _localback (`self.GetLocalBackSurface`))
        (return _localback)))
    (elif (and (> _returnvalue_7 _returnvalue_6) (> _returnvalue_7 _returnvalue_5))
      (if (> (`local.RightDot`) 0.0)
        (bind _localright (`self.GetLocalRightSurface`))
        (return _localright)
        (else
          (bind _localleft (`self.GetLocalLeftSurface`))
          (return _localleft)))
      (elif (> (`local.UpDot`) 0.0)
        (bind _localtop (`self.GetLocalTopSurface`))
        (return _localtop)
        (else
          (bind _localbottom (`self.GetLocalBottomSurface`))
          (return _localbottom))))))

(fn `IsGridPositionTaken`
  (params (GridPosition :type "/Game/LOGIC/Structures/F_Byte3 Structure"))
  (returns (IsTaken :type Boolean))
  (return (`self.IsGridPositionTakenMacro` GridPosition)))

(fn `RemoveTopSurface`)

(fn `UserConstructionScript`
  (set `self.GridGenerationCenter` (/ (- (`KismetMathLibrary.MakeVector` (`KismetMathLibrary.Conv_ByteToDouble` (`self.Depth`)) (`KismetMathLibrary.Conv_ByteToDouble` (`self.Width`)) (`KismetMathLibrary.Conv_ByteToDouble` (`self.Height`))) 1) 2)))