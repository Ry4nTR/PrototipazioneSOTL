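; Rounded cube world actor that measures how far the player has moved into its curved edge zone.
; The construction script derives the cube half-size from the mesh's X/Y bounds and scales it by a flat-zone ratio to get the edge threshold.
; Each tick converts the player's position to cube-local space and, when both X and Y lie in the edge band, prints the larger normalized 0–1 depth as debug output.
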(event `self.ReceiveBeginPlay`
  (`self.EnableInput` (`GameplayStatics.GetPlayerController` 0))
  (bind _asbp_third_person_character (cast `/Game/LOGIC/Blueprints/BP_ThirdPersonCharacter` (`GameplayStatics.GetPlayerCharacter` 0)))
  (set `self.PlayerRef` _asbp_third_person_character))

(event `self.ReceiveTick`
  (params (DeltaSeconds :type "Float (single-precision)"))
  (bind _distanceintocurve (`self.GetDistanceIntoCurve`))
  (`KismetSystemLibrary.PrintString` (`KismetStringLibrary.Conv_DoubleToString` _distanceintocurve)))

(fn `GetDistanceIntoCurve`
  (returns (DistanceIntoCurve :type "Float (double-precision)"))
  (bind _edgethreshold (`self.EdgeThreshold`))
  (bind _returnvalue (- (`self.CubeHalfSize`) (`self.EdgeThreshold`)))
  (bind _returnvalue_2 (`KismetMathLibrary.Abs` (.y (`KismetMathLibrary.InverseTransformLocation` (`SceneComponent.K2_GetComponentToWorld` (`self.RoundedCube`)) (`self.K2_GetActorLocation` (`self.PlayerRef`))))))
  (bind _returnvalue_3 (`KismetMathLibrary.Abs` (.x (`KismetMathLibrary.InverseTransformLocation` (`SceneComponent.K2_GetComponentToWorld` (`self.RoundedCube`)) (`self.K2_GetActorLocation` (`self.PlayerRef`))))))
  (if (and (> _returnvalue_3 _returnvalue) (> _returnvalue_2 _returnvalue))
    (return (`KismetMathLibrary.FMax` (`KismetMathLibrary.FClamp` (/ (- _returnvalue_3 _returnvalue) _edgethreshold)) (`KismetMathLibrary.FClamp` (/ (- _returnvalue_2 _returnvalue) _edgethreshold))))))

(fn `UserConstructionScript`
  (bind (_min _max) (break `Box` (`StaticMesh.GetBoundingBox` (`StaticMeshComponent.StaticMesh` (`self.RoundedCube`)))))
  (bind _output_get (set `self.CubeHalfSize` (`KismetMathLibrary.FMax` (.x (/ (- _max _min) 2)) (.y (/ (- _max _min) 2)))))
  (set `self.EdgeThreshold` (* _output_get (`self.FlatZoneRatio`))))