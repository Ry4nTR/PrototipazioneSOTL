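; BP_RubikGrid is an actor that builds a 3x3x3 Rubik's cube from BP_RubikNode actors.
; CreateGrid clears old nodes, then spawns, attaches and positions each node around a fixed centre, storing it in the Nodes map by grid coordinate.
; ColorNodeFaces derives outward face signs per axis, but its colour logic is disconnected.
; Nothing in this file calls CreateGrid or ColorNodeFaces, and the event graph is empty.
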(fn `ColorNodeFaces`
  (params (Node :type "/Game/LOGIC/Blueprints/BP_RubikNode Object Reference") (ByPosition :type "/Game/LOGIC/Structures/F_Byte3 Structure"))
  (locals (XFaceToColor :type "StaticMeshComponent Object Reference") (YFaceToColor :type "StaticMeshComponent Object Reference") (ZFaceToColor :type "StaticMeshComponent Object Reference") (XFaceColor :type "Color Structure") (YFaceColor :type "Color Structure") (ZFaceColor :type "Color Structure"))
  (set `/Game/LOGIC/Blueprints/BP_RubikNode.NormalFaces` (make `/Game/LOGIC/Structures/F_Int3` (select `byte` ByPosition_x_2_C11C5C0A456A85F6AE8A10AE086400B7 :`0` -1 :`1` 0 :`2` 1) (select `byte` ByPosition_y_5_F30064344551A26B705930A689FDADCE :`0` -1 :`1` 0 :`2` 1) (select `byte` ByPosition_z_6_0143F4DB433691C195BDE29DCE95AD98 :`0` -1 :`1` 0 :`2` 1)) Node))

(fn `CreateGrid`
  (locals (X :type Integer) (Y :type Integer) (Z :type Integer))
  (`self.DeleteGrid`)
  (for _index (range 3)
    (set `local.X` _index)
    (for _index_2 (range 3)
      (set `local.Y` _index_2)
      (for _index_3 (range 3)
        (set `local.Z` _index_3)
        (`self.CreateNodeAt` (make `/Game/LOGIC/Structures/F_Byte3` (`KismetMathLibrary.Conv_IntToByte` (`local.X`)) (`KismetMathLibrary.Conv_IntToByte` (`local.Y`)) (`KismetMathLibrary.Conv_IntToByte` (`local.Z`))))))))

(fn `CreateNodeAt`
  (params (Position :type "/Game/LOGIC/Structures/F_Byte3 Structure"))
  (locals (AddedNode :type "/Game/LOGIC/Blueprints/BP_RubikNode Object Reference"))
  (bind _returnvalue (`|SpawnActorFromClass` "/Game/LOGIC/Blueprints/BP_RubikNode.BP_RubikNode_C" (`self.GetTransform`) "Undefined" "MultiplyWithRoot" null null))
  (bind _output_get (set `local.AddedNode` _returnvalue))
  (`self.K2_AttachToActor` _output_get self "None" "KeepRelative" "KeepRelative" "KeepRelative" true)
  (`self.K2_SetActorRelativeTransform` (`local.AddedNode`) (`KismetMathLibrary.MakeTransform` (`self.GetNodeRelativePosition` (`local.Position`)) (struct) (`self.GetNodeRelativeScale`)) false true)
  (`BlueprintMapLibrary.Map_Add` (`self.Nodes`) (`local.Position`) (`local.AddedNode`)))

(fn `DeleteGrid`
  (locals (ToRemove :type "Array of /Game/LOGIC/Blueprints/BP_RubikNode Object Reference"))
  (bind _nodes (`self.Nodes`))
  (bind (_keypin _valuepin) (`|MapForEach` _nodes)
    (:`then`
      (`self.K2_DestroyActor` _valuepin))
    (:`CompletedPin`
      (`BlueprintMapLibrary.Map_Clear` _nodes))))

(fn `UserConstructionScript`
  ; old
  (set `self.GridGenerationCenter` (1.0 1.0 1.0)))