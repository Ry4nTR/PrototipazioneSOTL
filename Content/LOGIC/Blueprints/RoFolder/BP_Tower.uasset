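; BP_Tower is a tower attached to a Rubik node that turns hit locations into rotation requests for that node.
; ProcessHitAtLocation projects the offset from the tower to the hit onto the plane of FaceNormal, ignoring near-central hits.
; The normalized in-plane direction and face normal go to the node's RequestRotateFromFaceMessage, alongside a temporary debug arrow showing that direction.
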(fn `ProcessHitAtLocation`
  (params (HitLocation :type "Vector Structure"))
  (locals (HitDir :type "Vector Structure") (proj :type "Vector Structure"))
  (bind _returnvalue (`self.K2_GetActorLocation`))
  (bind _output_get (set `local.HitDir` (- HitLocation (`self.K2_GetActorLocation`))))
  (bind _returnvalue_2 (- _output_get (* (`self.FaceNormal`) (`KismetMathLibrary.Dot_VectorVector` _output_get (`self.FaceNormal`)))))
  (set `local.proj` _returnvalue_2)
  (if (> (`KismetMathLibrary.VSize` _returnvalue_2) 1.0)
    (`KismetSystemLibrary.DrawDebugArrow` _returnvalue (* (+ _returnvalue (`KismetMathLibrary.Normal` (`local.proj`))) 100.0) 0.0 (struct :`R` 1.0 :`G` 1.0 :`A` 1.0) 3.0 2.0)
    (message `/Game/LOGIC/Blueprints/RoFolder/RBI_RubikInterface.RequestRotateFromFace` (`self.AttachedRubikNode`) (`self.FaceNormal`) (`KismetMathLibrary.Normal` (`local.proj`)))))

(fn `UserConstructionScript`)