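; Falling cube for a Tetris-style 3D grid, dropping toward BP_Grid along an axis chosen by its Face.
; InitFallingCube randomizes its cell, offsets it along that axis and spawns another BP_FallingNode.
; Axis indices keep the math face-agnostic; Tick uses separate VInterpTo speeds for falling and lateral motion.
; MoveAlongGrid shifts clamped plane cells unless near the surface; landing and grid-registration logic is unwired.
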(event `InitFallingCube`
  (bind _returnvalue (`GameplayStatics.GetActorOfClass` "/Game/LOGIC/Blueprints/NICK/BP_Grid.BP_Grid_C"))
  (set `self.Grid` _returnvalue)
  (set `self.Face` "NewEnumerator0")
  (set `self.GridSize` (5.0 5.0 5.0))
  (set `self.CubeScale ` 25.0)
  (set `self.SpawnHeightOffset` 50000.0)
  (`self.SetPositionFallingNode`)
  (`|SpawnActorFromClass` "BP_FallingNode_C" (`KismetMathLibrary.Conv_VectorToTransform` (0.0 0.0 0.0)) "Undefined" "MultiplyWithRoot" null null))

(event `self.ReceiveBeginPlay`
  (`self.SettingFallingAxis`))

(event `self.ReceiveTick`
  (params (DeltaSeconds :type "Float (single-precision)"))
  (if (`self.FirstTime`)
    (set `self.FirstTime` false)
    (else
      (`self.SmoothUpdateActorLocation`))))

(fn `CheckProximityToSurfaceLayer `
  (bind (_returnvalue_x _returnvalue_y _returnvalue_z) (`KismetMathLibrary.BreakVector` (`self.K2_GetActorLocation`)))
  (bind _layerfacingaxisondepth (`/Game/LOGIC/Blueprints/NICK/BP_Grid.GetLocalLayerFacingAxis` (`self.Grid`) (`self.FallingAxisIndex`) 4))
  (bind (_keypin _valuepin) (`|MapForEach` _layerfacingaxisondepth :!label _label)
    (:`then`
      (bind (_returnvalue_x_2 _returnvalue_y_2 _returnvalue_z_2) (`KismetMathLibrary.BreakVector` (`self.K2_GetActorLocation` _valuepin)))
      (if (< (- (`|GetArrayItem` (`|MakeArray` _returnvalue_x _returnvalue_y _returnvalue_z) (`KismetMathLibrary.Conv_ByteToInt` (`self.FallingAxisIndex`))) (`|GetArrayItem` (`|MakeArray` _returnvalue_x_2 _returnvalue_y_2 _returnvalue_z_2) (`KismetMathLibrary.Conv_ByteToInt` (`self.FallingAxisIndex`)))) (`self.SurfaceProximityLockDistance`))
        (set `self.isNearSurface` true)
        (goto _label :!via `BreakPin`)
        (else
          (set `self.isNearSurface` false)
          (goto _label :!via `BreakPin`))))))

(fn `CombineInterpolatedLocationAxes`
  (returns (CombinedVector :type "Vector Structure"))
  (locals (FinalArray :type "Array of Float (double-precision)"))
  (bind (_planeaxis1 _planeaxis2) (`self.LateralTargetInterpolation`))
  (bind (_x _y _z) (`self.GetArrayElemFromArray` (`local.FinalArray`)))
  (set `local.FinalArray` (`|MakeArray` 0.0 0.0 0.0))
  (`KismetArrayLibrary.Array_Set` (`local.FinalArray`) (`KismetMathLibrary.Conv_ByteToInt` (`self.PlaneAxis1Index`)) _planeaxis1)
  (`KismetArrayLibrary.Array_Set` (`local.FinalArray`) (`KismetMathLibrary.Conv_ByteToInt` (`self.PlaneAxis2Index`)) _planeaxis2)
  (`KismetArrayLibrary.Array_Set` (`local.FinalArray`) (`KismetMathLibrary.Conv_ByteToInt` (`self.FallingAxisIndex`)) (`self.FallingTargetInterpolation`))
  (return (`KismetMathLibrary.MakeVector` _x _y _z)))

(fn `GetFallingAxis`
  (returns (`DirectionSign ` :type "Float (double-precision)"))
  (switch `/Game/LOGIC/Blueprints/RO/Tetris/WorldFaces` (`self.Face`)
    (:`NewEnumerator0`
      (return 1.0))
    (:`NewEnumerator1`
      (return -1.0))
    (:`NewEnumerator2`
      (return 1.0))
    (:`NewEnumerator3`
      (return -1.0))
    (:`NewEnumerator4`
      (return 1.0))
    (:`NewEnumerator5`
      (return -1.0))))

(fn `MoveAlongGrid`
  (params (Direction :type "Vector Structure"))
  (locals (MoveCubeArray :type "Array of Float (double-precision)") (PositionArray :type "Array of Float (double-precision)") (DirectionArray :type "Array of Float (double-precision)"))
  (bind (_gridposition_x _gridposition_y _gridposition_z) (`KismetMathLibrary.BreakVector` (`self.GridPosition`)))
  (bind (_planeaxis1 _planeaxis2) (`self.GetPlaneAxisFromArray` (`local.DirectionArray`)))
  (bind (_planeaxis1_2 _planeaxis2_2) (`self.GetPlaneAxisFromArray` (`local.PositionArray`)))
  (bind (_planeaxis1_3 _planeaxis2_3) (`self.GetPlaneAxisFromVector` (`self.GridSize`)))
  (bind (_x _y _z) (`self.GetArrayElemFromArray` (`local.PositionArray`)))
  (`self.CheckProximityToSurfaceLayer `)
  (if (not (`self.isNearSurface`))
    (set `local.DirectionArray` (`|MakeArray` Direction_X Direction_Y Direction_Z))
    (set `local.PositionArray` (`|MakeArray` _gridposition_x _gridposition_y _gridposition_z))
    (`KismetArrayLibrary.Array_Set` (`local.PositionArray`) (`KismetMathLibrary.Conv_ByteToInt` (`self.PlaneAxis1Index`)) (`KismetMathLibrary.FClamp` (+ _planeaxis1_2 _planeaxis1) 0.0 (- _planeaxis1_3 1.0)))
    (`KismetArrayLibrary.Array_Set` (`local.PositionArray`) (`KismetMathLibrary.Conv_ByteToInt` (`self.PlaneAxis2Index`)) (`KismetMathLibrary.FClamp` (+ _planeaxis2_2 _planeaxis2) 0.0 (- _planeaxis2_3 1.0)))
    (set `self.GridPosition` (`KismetMathLibrary.MakeVector` _x _y _z))
    (`self.UpdateTargetWorldLocation`)))

(fn `SetByteGridPosition`
  (locals (ByteGridPosition :type "Array of Byte"))
  (bind (_planeaxis1 _planeaxis2) (`self.GetPlaneAxisFromArray` (`self.GridPosArray`)))
  (bind (_x _y _z) (`self.GetArrayElemFromArray` (`local.ByteGridPosition`)))
  (set `local.ByteGridPosition` (`|MakeArray` 0 0 0))
  (`KismetArrayLibrary.Array_Set` (`local.ByteGridPosition`) (`KismetMathLibrary.Conv_ByteToInt` (`self.FallingAxisIndex`)) (`KismetMathLibrary.Conv_IntToByte` (`self.CurrentFallingGridPosition`)))
  (`KismetArrayLibrary.Array_Set` (`local.ByteGridPosition`) (`KismetMathLibrary.Conv_ByteToInt` (`self.PlaneAxis1Index`)) (`KismetMathLibrary.Conv_Int64ToByte` (`KismetMathLibrary.Conv_DoubleToInt64` _planeaxis1)))
  (`KismetArrayLibrary.Array_Set` (`local.ByteGridPosition`) (`KismetMathLibrary.Conv_ByteToInt` (`self.PlaneAxis2Index`)) (`KismetMathLibrary.Conv_Int64ToByte` (`KismetMathLibrary.Conv_DoubleToInt64` _planeaxis2)))
  (set `self.ByteGridPostion` (make `/Game/LOGIC/Structures/F_Byte3` _x _y _z)))

(fn `SetPositionFallingNode`
  (bind (_x _y _z) (`self.GetArrayElemFromArray` (`self.PositionArray`)))
  (bind (_x_2 _y_2 _z_2) (`self.GetArrayElemFromArray` (`self.PositionArray`)))
  (bind (_planeaxis1 _planeaxis2) (`self.GetPlaneAxisFromVector` (`self.GridSize`)))
  (bind (_x_3 _y_3 _z_3) (`self.GetArrayElemFromArray` (`self.WorldPosArray`)))
  (bind (_gridoffset_x _gridoffset_y _gridoffset_z) (`KismetMathLibrary.BreakVector` (`/Game/LOGIC/Blueprints/NICK/BP_Grid.GetLocalOffsetFromCenter` (`self.Grid`) (make `/Game/LOGIC/Structures/F_Byte3` (`KismetMathLibrary.Conv_IntToByte` _x) (`KismetMathLibrary.Conv_IntToByte` _y) (`KismetMathLibrary.Conv_IntToByte` _z)))))
  (`self.SettingFallingAxis`)
  (set `self.PositionArray` (`|MakeArray` 0 0 0))
  (`KismetArrayLibrary.Array_Set` (`self.PositionArray`) (`KismetMathLibrary.Conv_ByteToInt` (`self.PlaneAxis1Index`)) (`KismetMathLibrary.RandomIntegerInRange` 0 (- (`KismetMathLibrary.FTrunc` _planeaxis1) 1)))
  (`KismetArrayLibrary.Array_Set` (`self.PositionArray`) (`KismetMathLibrary.Conv_ByteToInt` (`self.PlaneAxis2Index`)) (`KismetMathLibrary.RandomIntegerInRange` 0 (- (`KismetMathLibrary.FTrunc` _planeaxis2) 1)))
  (set `self.GridPosition` (`KismetMathLibrary.MakeVector` (`KismetMathLibrary.Conv_IntToDouble` _x_2) (`KismetMathLibrary.Conv_IntToDouble` _y_2) (`KismetMathLibrary.Conv_IntToDouble` _z_2)))
  (set `self.WorldPosArray` (`|MakeArray` _gridoffset_x _gridoffset_y _gridoffset_z))
  (bind _directionsign_ (`self.GetFallingAxis`))
  (`KismetArrayLibrary.Array_Set` (`self.WorldPosArray`) (`KismetMathLibrary.Conv_ByteToInt` (`self.FallingAxisIndex`)) (+ (`|GetArrayItem` (`self.WorldPosArray`) (`KismetMathLibrary.Conv_ByteToInt` (`self.FallingAxisIndex`))) (* _directionsign_ (`self.SpawnHeightOffset`))))
  (`self.K2_SetActorLocation` (`KismetMathLibrary.MakeVector` _x_3 _y_3 _z_3))
  (`self.SetActorScale3D` (`KismetMathLibrary.Conv_DoubleToVector` (`self.CubeScale `)))
  (set `self.IsFalling` true)
  (`self.UpdateTargetWorldLocation`))

(fn `SettingFallingAxis`
  (switch `/Game/LOGIC/Blueprints/RO/Tetris/WorldFaces` (`self.Face`)
    (:`NewEnumerator0`
      (set `self.FallingAxisIndex` 2)
      (set `self.PlaneAxis1Index` 0)
      (set `self.PlaneAxis2Index` 1))
    (:`NewEnumerator1`
      (set `self.FallingAxisIndex` 2)
      (set `self.PlaneAxis1Index` 0)
      (set `self.PlaneAxis2Index` 1))
    (:`NewEnumerator2`
      (set `self.FallingAxisIndex` 1)
      (set `self.PlaneAxis1Index` 0)
      (set `self.PlaneAxis2Index` 2))
    (:`NewEnumerator3`
      (set `self.FallingAxisIndex` 1)
      (set `self.PlaneAxis1Index` 0)
      (set `self.PlaneAxis2Index` 2))
    (:`NewEnumerator4`
      (set `self.FallingAxisIndex` 0)
      (set `self.PlaneAxis1Index` 1)
      (set `self.PlaneAxis2Index` 2))
    (:`NewEnumerator5`
      (set `self.FallingAxisIndex` 0)
      (set `self.PlaneAxis1Index` 1)
      (set `self.PlaneAxis2Index` 2))))

(fn `ShouldStopFalling`
  (returns (`ShouldStop ` :type Boolean))
  (locals (ByteGridPositio :type "Array of Byte"))
  (bind (_returnvalue_x _returnvalue_y _returnvalue_z) (`KismetMathLibrary.BreakVector` (`self.K2_GetActorLocation`)))
  (bind (_planeaxis1 _planeaxis2) (`self.GetPlaneAxisFromArray` (`self.GridPosArray`)))
  (bind (_x _y _z) (`self.GetArrayElemFromArray` (`local.ByteGridPositio`)))
  (bind _output_get (set `self.CurrentFallingGridPosition` (`KismetMathLibrary.Round` (/ (`|GetArrayItem` (`|MakeArray` _returnvalue_x _returnvalue_y _returnvalue_z) (`KismetMathLibrary.Conv_ByteToInt` (`self.FallingAxisIndex`))) (`self.CubeScale `)))))
  (set `local.ByteGridPositio` (`|MakeArray` 0 0 0))
  (`KismetArrayLibrary.Array_Set` (`local.ByteGridPositio`) (`KismetMathLibrary.Conv_ByteToInt` (`self.FallingAxisIndex`)) (`KismetMathLibrary.Conv_IntToByte` (- _output_get 1)))
  (`KismetArrayLibrary.Array_Set` (`local.ByteGridPositio`) (`KismetMathLibrary.Conv_ByteToInt` (`self.PlaneAxis1Index`)) (`KismetMathLibrary.Conv_Int64ToByte` (`KismetMathLibrary.Conv_DoubleToInt64` _planeaxis1)))
  (`KismetArrayLibrary.Array_Set` (`local.ByteGridPositio`) (`KismetMathLibrary.Conv_ByteToInt` (`self.PlaneAxis2Index`)) (`KismetMathLibrary.Conv_Int64ToByte` (`KismetMathLibrary.Conv_DoubleToInt64` _planeaxis2)))
  (bind _istaken (`/Game/LOGIC/Blueprints/NICK/BP_Grid.IsGridPositionTaken` (`self.Grid`) (make `/Game/LOGIC/Structures/F_Byte3` _x _y _z)))
  (return _istaken))

(fn `SmoothUpdateActorLocation`
  (locals (UpdateMovementArray :type "Array of Float (double-precision)"))
  (if (`self.IsFalling`)
    (bind _combinedvector (`self.CombineInterpolatedLocationAxes`))
    (`self.K2_SetActorLocation` _combinedvector)))

(fn `UpdateTargetWorldLocation`
  (locals (FallingOffsetArray :type "Array of Integer") (ActorLocationArray :type "Array of Float (double-precision)"))
  (bind (_returnvalue_x _returnvalue_y _returnvalue_z) (`KismetMathLibrary.BreakVector` (`self.K2_GetActorLocation`)))
  (bind (_x _y _z) (`self.GetArrayElemFromVector` (`self.GridPosition`)))
  (bind (_x_2 _y_2 _z_2) (`self.GetArrayElemFromArray` (`local.ActorLocationArray`)))
  (bind (_x_3 _y_3 _z_3) (`self.GetArrayElemFromArray` (`local.ActorLocationArray`)))
  (bind (_gridoffset_x _gridoffset_y _gridoffset_z) (`KismetMathLibrary.BreakVector` (`/Game/LOGIC/Blueprints/NICK/BP_Grid.GetLocalOffsetFromCenter` (`self.Grid`) (make `/Game/LOGIC/Structures/F_Byte3` (`KismetMathLibrary.Conv_Int64ToByte` (`KismetMathLibrary.Conv_DoubleToInt64` _x)) (`KismetMathLibrary.Conv_Int64ToByte` (`KismetMathLibrary.Conv_DoubleToInt64` _y)) (`KismetMathLibrary.Conv_Int64ToByte` (`KismetMathLibrary.Conv_DoubleToInt64` _z))))))
  (bind _array (`|MakeArray` _gridoffset_x _gridoffset_y _gridoffset_z))
  (bind (_planeaxis1 _planeaxis2) (`self.GetPlaneAxisFromArray` _array))
  (set `local.ActorLocationArray` (`|MakeArray` _returnvalue_x _returnvalue_y _returnvalue_z))
  (`KismetArrayLibrary.Array_Set` (`local.ActorLocationArray`) (`KismetMathLibrary.Conv_ByteToInt` (`self.PlaneAxis1Index`)) _planeaxis1)
  (`KismetArrayLibrary.Array_Set` (`local.ActorLocationArray`) (`KismetMathLibrary.Conv_ByteToInt` (`self.PlaneAxis2Index`)) _planeaxis2)
  (set `self.LateralTargetLocation` (`KismetMathLibrary.MakeVector` _x_3 _y_3 _z_3))
  (`KismetArrayLibrary.Array_Set` (`local.ActorLocationArray`) (`KismetMathLibrary.Conv_ByteToInt` (`self.FallingAxisIndex`)) (`|GetArrayItem` _array (`KismetMathLibrary.Conv_ByteToInt` (`self.FallingAxisIndex`))))
  (set `self.FallingTargetLocation` (`KismetMathLibrary.MakeVector` _x_2 _y_2 _z_2)))

(fn `UserConstructionScript`)