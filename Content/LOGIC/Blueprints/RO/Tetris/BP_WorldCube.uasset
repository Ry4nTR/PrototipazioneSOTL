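; BP_WorldCube is an actor in the Tetris folder that builds a flat grid of static mesh components.
; Its Construction Script loops over GridSize X and Y, placing each component on the XY plane at CubeScale spacing.
; Each cell also gets a thick red debug box, drawn at the same coordinates in world space without the actor's transform.
; The event graph holds no gameplay logic.
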(event `self.ReceiveBeginPlay`)

(fn `UserConstructionScript`
  (bind _cubescale_ (`self.CubeScale `))
  (bind (_x _y) (`KismetMathLibrary.BreakVector2D` (`self.GridSize `)))
  (bind _returnvalue (/ (`self.CubeScale `) 2.0))
  (for _index (range (+ (`KismetMathLibrary.FTrunc` (- _x 1.0)) 1))
    (for _index_2 (range (+ (`KismetMathLibrary.FTrunc` (- _y 1.0)) 1))
      (bind _returnvalue_2 (`AddComponent|NODE_AddStaticMeshComponent-0`))
      (bind _output_get (set `self.CubeComponent ` _returnvalue_2))
      (bind _returnvalue_3 (`KismetMathLibrary.MakeVector` (* (`KismetMathLibrary.Conv_IntToDouble` _index) _cubescale_) (* _cubescale_ (`KismetMathLibrary.Conv_IntToDouble` _index_2))))
      (`SceneComponent.K2_SetRelativeLocation` _output_get _returnvalue_3 false false)
      (`KismetSystemLibrary.DrawDebugBox` _returnvalue_3 (`KismetMathLibrary.MakeVector` _returnvalue _returnvalue 5.0) (struct :`R` 1.0 :`A` 1.0) (struct) 0.0 100.0))))