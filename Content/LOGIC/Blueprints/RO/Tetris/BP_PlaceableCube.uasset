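; BP_PlaceableCube is a grid-based falling cube actor for a Tetris-style game, apparently work in progress.
; Tick lowers GridPosition.Z and sets the rounded location, but an always-true branch immediately locks and snaps it, then interpolates toward TargetWorldLocation once.
; UpdateWorldLocation derives that target from CubeScale with a fixed height and prints it.
; MoveCube zeroes GridPosition, leaving its Direction clamping logic unconnected.
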(event `self.ReceiveBeginPlay`
  (set `self.GravityDirection` (0.0 0.0 -1.0)))

(event `self.ReceiveTick`
  (params (DeltaSeconds :type "Float (single-precision)"))
  (bind _gridunitsize (`self.GridUnitSize`))
  (if (not (`self.IsLocked`))
    (bind _output_get (set `self.GridPosition` (`KismetMathLibrary.MakeVector` 0.0 0.0 (- (.z (`self.GridPosition`)) (/ (.z (* (`self.FallSpeed`) (`GameplayStatics.GetWorldDeltaSeconds`))) (`self.GridUnitSize`))))))
    (`self.UpdateWorldLocation`)
    (`self.K2_SetActorLocation` (`KismetMathLibrary.MakeVector` (* (.x _output_get) _gridunitsize) (* (.y _output_get) _gridunitsize) (* (`KismetMathLibrary.Conv_IntToDouble` (`KismetMathLibrary.Round` (.z _output_get))) _gridunitsize)))
    (if true
      (`self.LockToGrid`)
      (`self.K2_SetActorLocation` (`KismetMathLibrary.VInterpTo` (`self.K2_GetActorLocation`) (`self.TargetWorldLocation `) (`GameplayStatics.GetWorldDeltaSeconds`) 3.0)))))

(fn `LockToGrid`
  (set `self.IsLocked` true)
  (bind _newlocation (`self.SnapToGrid` (`self.K2_GetActorLocation`)))
  (`self.K2_SetActorLocation` _newlocation))

(fn `MoveCube`
  (params (Direction :type "Vector Structure"))
  (if (not (`self.IsLocked`))
    (set `self.GridPosition` (0.0 0.0 0.0))
    (`self.UpdateWorldLocation`)))

(fn `SnapToGrid`
  (params (InputLocation :type "Vector Structure"))
  (returns (NewLocation :type "Vector Structure"))
  (bind _gridunitsize (`self.GridUnitSize`))
  (bind _gridunitsize_2 (`self.GridUnitSize`))
  (return (`KismetMathLibrary.MakeVector` (* (`KismetMathLibrary.Round` (/ (.x InputLocation) _gridunitsize_2)) _gridunitsize) (* (`KismetMathLibrary.Round` (/ (.y InputLocation) _gridunitsize_2)) _gridunitsize) (* (`KismetMathLibrary.Round` (/ (.z InputLocation) _gridunitsize_2)) _gridunitsize))))

(fn `UpdateWorldLocation`
  (bind _cubescale_ (`self.CubeScale `))
  (bind _returnvalue (* (.x (`self.GridPosition`)) _cubescale_))
  (bind _returnvalue_2 (* _cubescale_ (.y (`self.GridPosition`))))
  (set `self.TargetWorldLocation ` (`KismetMathLibrary.MakeVector` _returnvalue _returnvalue_2 50000.0))
  (`KismetSystemLibrary.PrintString` (`KismetStringLibrary.Concat_StrStr` "Current block position" "X: " (`KismetStringLibrary.Conv_DoubleToString` _returnvalue) "Y:" (`KismetStringLibrary.Conv_DoubleToString` _returnvalue_2))))

(fn `UserConstructionScript`)