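; Falling cube actor for a 3D Tetris-style grid, whose Face sets which axis it falls along and which two axes it moves on.
; Each tick lowers GridPosition along the fall axis, eases the actor toward the scaled position and locks it when Grid.Nodes contains the next cell.
; MoveCube shifts it in the plane without bounds clamping.
; Opposite faces share the same negative fall direction, and locking does not write to the grid.
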(event `self.ReceiveBeginPlay`
  (`self.InitializeFallingLogic`))

(event `self.ReceiveTick`
  (params (DeltaSeconds :type "Float (single-precision)"))
  (`self.UpdateMovement`))

(fn `InitializeFallingLogic`
  (switch `/Game/LOGIC/Blueprints/RO/Tetris/WorldFaces` (`self.Face`)
    (:`NewEnumerator0`
      (set `self.FallingAxisIndex` 2)
      (set `self.PlaneAxis1Index` 0)
      (set `self.PlaneAxis2Index` 1))
    (:`NewEnumerator1`
      (set `self.FallingAxisIndex` 2)
      (set `self.PlaneAxis1Index` 0)
      (set `self.PlaneAxis2Index` 1))
    (:`NewEnumerator2`
      (set `self.FallingAxisIndex` 0)
      (set `self.PlaneAxis1Index` 1)
      (set `self.PlaneAxis2Index` 2))
    (:`NewEnumerator3`
      (set `self.FallingAxisIndex` 0)
      (set `self.PlaneAxis1Index` 1)
      (set `self.PlaneAxis2Index` 2))
    (:`NewEnumerator4`
      (set `self.FallingAxisIndex` 1)
      (set `self.PlaneAxis1Index` 0)
      (set `self.PlaneAxis2Index` 2))
    (:`NewEnumerator5`
      (set `self.FallingAxisIndex` 1)
      (set `self.PlaneAxis1Index` 0)
      (set `self.PlaneAxis2Index` 2))))

(fn `LockToGrid`
  (bind (_gridposition_x _gridposition_y _gridposition_z) (`KismetMathLibrary.BreakVector` (`self.GridPosition`)))
  (set `self.IsFalling` false)
  (`self.K2_SetActorLocation` (`self.TargetWorldLocation `))
  (`KismetSystemLibrary.PrintString` (`KismetStringLibrary.Concat_StrStr` (`KismetStringLibrary.Conv_ByteToString` (`KismetMathLibrary.Conv_Int64ToByte` (`KismetMathLibrary.Conv_DoubleToInt64` _gridposition_x))) ", " (`KismetStringLibrary.Conv_ByteToString` (`KismetMathLibrary.Conv_Int64ToByte` (`KismetMathLibrary.Conv_DoubleToInt64` _gridposition_y))) ", " (`KismetStringLibrary.Conv_ByteToString` (`KismetMathLibrary.Conv_Int64ToByte` (`KismetMathLibrary.Conv_DoubleToInt64` _gridposition_z))) "    LOCKED AT THIS GRIDPOSITION")))

(fn `MoveCube`
  (params (Direction :type "Vector Structure"))
  (locals (MoveCubeArray :type "Array of Float (double-precision)"))
  (bind _movecubearray (`local.MoveCubeArray`))
  (bind _movecubearray_2 (`local.MoveCubeArray`))
  (bind (_gridposition_x _gridposition_y _gridposition_z) (`KismetMathLibrary.BreakVector` (`self.GridPosition`)))
  (bind _returnvalue (`KismetMathLibrary.Conv_ByteToInt` (`self.PlaneAxis1Index`)))
  (bind _returnvalue_2 (`KismetMathLibrary.Conv_ByteToInt` (`self.PlaneAxis2Index`)))
  (set `local.MoveCubeArray` (`|MakeArray` _gridposition_x _gridposition_y _gridposition_z))
  (`KismetArrayLibrary.Array_Set` (`local.MoveCubeArray`) _returnvalue (+ (.x Direction) (`|GetArrayItem` _movecubearray_2 _returnvalue)))
  (`KismetArrayLibrary.Array_Set` (`local.MoveCubeArray`) _returnvalue_2 (+ (.y Direction) (`|GetArrayItem` _movecubearray_2 _returnvalue_2)))
  (set `self.GridPosition` (`KismetMathLibrary.MakeVector` (`|GetArrayItem` _movecubearray) (`|GetArrayItem` _movecubearray 1) (`|GetArrayItem` _movecubearray 2)))
  (`self.UpdateTargetWorldLocation`))

(fn `UpdateMovement`
  (locals (UpdateMovementArray :type "Array of Float (double-precision)"))
  (bind _updatemovementarray (`local.UpdateMovementArray`))
  (bind _updatemovementarray_2 (`local.UpdateMovementArray`))
  (bind (_gridsize_x _gridsize_y _gridsize_z) (`KismetMathLibrary.BreakVector` (`self.GridSize`)))
  (bind (_gridposition_x _gridposition_y _gridposition_z) (`KismetMathLibrary.BreakVector` (`self.GridPosition`)))
  (bind _returnvalue (`KismetMathLibrary.Conv_ByteToInt` (`self.FallingAxisIndex`)))
  (if (`self.IsFalling`)
    (bind _output_get (set `local.UpdateMovementArray` (`|MakeArray` _gridposition_x _gridposition_y _gridposition_z)))
    (`KismetArrayLibrary.Array_Set` (`local.UpdateMovementArray`) _returnvalue (- (`|GetArrayItem` _output_get _returnvalue) (* (`self.FallingSpeed `) (`GameplayStatics.GetWorldDeltaSeconds`))))
    (set `self.GridPosition` (`KismetMathLibrary.MakeVector` (`|GetArrayItem` _updatemovementarray) (`|GetArrayItem` _updatemovementarray 1) (`|GetArrayItem` _updatemovementarray 2)))
    (`self.UpdateTargetWorldLocation`)
    (`self.K2_SetActorLocation` (`KismetMathLibrary.VInterpTo` (`self.K2_GetActorLocation`) (`self.TargetWorldLocation `) (`GameplayStatics.GetWorldDeltaSeconds`) 3.0))
    (`KismetArrayLibrary.Array_Set` (`local.UpdateMovementArray`) (`KismetMathLibrary.Conv_ByteToInt` (`self.FallingAxisIndex`)) (`KismetMathLibrary.FClamp` (- (`|GetArrayItem` (`local.UpdateMovementArray`) (`KismetMathLibrary.Conv_ByteToInt` (`self.FallingAxisIndex`))) 1.0) 0.0 (- (`|GetArrayItem` (`|MakeArray` _gridsize_x _gridsize_y _gridsize_z) (`KismetMathLibrary.Conv_ByteToInt` (`self.FallingAxisIndex`))) 1.0)))
    (bind _output_get_2 (set `self.NextCellKey` (make `/Game/LOGIC/Structures/F_Byte3` (`KismetMathLibrary.Conv_Int64ToByte` (`KismetMathLibrary.Conv_DoubleToInt64` (`|GetArrayItem` _updatemovementarray_2))) (`KismetMathLibrary.Conv_Int64ToByte` (`KismetMathLibrary.Conv_DoubleToInt64` (`|GetArrayItem` _updatemovementarray_2 1))) (`KismetMathLibrary.Conv_Int64ToByte` (`KismetMathLibrary.Conv_DoubleToInt64` (`|GetArrayItem` _updatemovementarray_2 2))))))
    (if (`BlueprintMapLibrary.Map_Contains` (`/Game/LOGIC/Blueprints/NICK/BP_Grid.Nodes` (`self.Grid`)) _output_get_2)
      (`self.LockToGrid`))))

(fn `UpdateTargetWorldLocation`
  (bind _cubescale_ (`self.CubeScale `))
  (set `self.TargetWorldLocation ` (`KismetMathLibrary.MakeVector` (* (.x (`self.GridPosition`)) _cubescale_) (* (.y (`self.GridPosition`)) _cubescale_) (* (.z (`self.GridPosition`)) _cubescale_))))

(fn `UserConstructionScript`)