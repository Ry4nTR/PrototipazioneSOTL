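; Rounded cube actor that rotates its mesh as the player pawn moves through the curved edge zone around its faces.
; Construction derives the edge threshold from mesh bounds and a flat-zone ratio.
; Each tick, the pawn's mesh-local X/Y position gives a normalized curve progress and a dominant-side axis.
; Progress change times a maximum angle builds the target, and the RInterpTo result is passed to AddWorldRotation as a delta.
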(event `self.ReceiveBeginPlay`
  (set `self.PlayerPawn` (`GameplayStatics.GetPlayerPawn` 0))
  (bind _distanceintocurve_ (`self.GetDistanceIntoCurve`))
  (set `self.LastDistanceIntoCurve` _distanceintocurve_))

(event `self.ReceiveTick`
  (params (DeltaSeconds :type "Float (single-precision)"))
  (if (`KismetSystemLibrary.IsValid` (`self.PlayerPawn`))
    (bind _rotationdirection (`self.GetRotationDirection`))
    (bind _distanceintocurve_ (`self.GetDistanceIntoCurve`))
    (`self.RotateByCurveProgress` _rotationdirection _distanceintocurve_ DeltaSeconds)
    (set `self.LastDistanceIntoCurve` _distanceintocurve_)))

(fn `GetDistanceIntoCurve`
  (returns (`DistanceIntoCurve ` :type "Float (double-precision)"))
  (bind _returnvalue (- (`self.CubeHalfSize`) (`self.EdgeThreshold`)))
  (bind _output_get (set `self.DeltaX` (`KismetMathLibrary.FMax` 0.0 (- (`KismetMathLibrary.Abs` (.x (`KismetMathLibrary.InverseTransformLocation` (`SceneComponent.K2_GetComponentToWorld` (`self.Mesh`)) (`self.K2_GetActorLocation` (`self.PlayerPawn`))))) _returnvalue))))
  (bind _output_get_2 (set `self.DeltaY` (`KismetMathLibrary.FMax` 0.0 (- (`KismetMathLibrary.Abs` (.y (`KismetMathLibrary.InverseTransformLocation` (`SceneComponent.K2_GetComponentToWorld` (`self.Mesh`)) (`self.K2_GetActorLocation` (`self.PlayerPawn`))))) _returnvalue))))
  (return (`KismetMathLibrary.FMax` (`KismetMathLibrary.FClamp` (/ _output_get_2 (`self.EdgeThreshold`))) (`KismetMathLibrary.FClamp` (/ _output_get (`self.EdgeThreshold`))))))

(fn `GetRotationDirection`
  (returns (RotationDirection :type "Vector Structure"))
  (bind _x (.x (`KismetMathLibrary.InverseTransformLocation` (`SceneComponent.K2_GetComponentToWorld` (`self.Mesh`)) (`self.K2_GetActorLocation` (`self.PlayerPawn`)))))
  (bind _y (.y (`KismetMathLibrary.InverseTransformLocation` (`SceneComponent.K2_GetComponentToWorld` (`self.Mesh`)) (`self.K2_GetActorLocation` (`self.PlayerPawn`)))))
  (if (> (`KismetMathLibrary.Abs` _x) (`KismetMathLibrary.Abs` _y))
    (if (> _x 0.0)
      (return (0.0 -1.0 0.0))
      (else
        (return (0.0 1.0 0.0))))
    (elif (> _y 0.0)
      (return (1.0 0.0 0.0))
      (else
        (return (-1.0 0.0 0.0))))))

(fn `RotateByCurveProgress`
  (params (RotationDirection :type "Vector Structure") (`CurrentDistance ` :type "Float (double-precision)") (DeltaSec :type "Float (double-precision)"))
  (bind _returnvalue (`SceneComponent.K2_GetComponentRotation` (`self.Mesh`)))
  (if (and (> `CurrentDistance ` 0.0) (< `CurrentDistance ` 1.0))
    (bind _output_get (set `self.TargetRotation` (`KismetMathLibrary.ComposeRotators` _returnvalue (`KismetMathLibrary.RotatorFromAxisAndAngle` RotationDirection (* (- `CurrentDistance ` (`self.LastDistanceIntoCurve`)) (`self.MaxCurveAngle`))))))
    (`SceneComponent.K2_AddWorldRotation` (`self.Mesh`) (`KismetMathLibrary.RInterpTo` _returnvalue _output_get DeltaSec (`self.InterpSpeed `)) false false)))

(fn `UserConstructionScript`
  (bind (_min _max) (break `Box` (`StaticMesh.GetBoundingBox` (`StaticMeshComponent.StaticMesh` (`self.Mesh`)))))
  (bind _returnvalue (- _max _min))
  (`parent.UserConstructionScript`)
  (bind _output_get (set `self.CubeExtent` (* _returnvalue 0.5)))
  (set `self.CubeRadius` (`KismetMathLibrary.FMax` (.x _output_get) (.y _output_get)))
  (bind _output_get_2 (set `self.CubeHalfSize` (`KismetMathLibrary.FMax` (.x (/ _returnvalue 2.0)) (.y (/ _returnvalue 2.0)))))
  (set `self.EdgeThreshold` (* _output_get_2 (- 1.0 (`self.FlatZoneRatio`)))))