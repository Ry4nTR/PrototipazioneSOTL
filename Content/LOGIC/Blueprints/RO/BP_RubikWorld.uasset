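; Rubik-style world actor that, on pressing E, rolls the sky sphere and every cube except the player's current base cube by 90 degrees.
; Start and target rotations are cached in parallel arrays, then a timeline lerps each component between them, bracketed by root-shake timelines.
; The rotation axis is set on the third-person character at the start and zeroed during the closing shake.
; RotateComponent is an empty stub.
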(event `self.ReceiveBeginPlay`
  (`self.EnableInput` (`GameplayStatics.GetPlayerController` 0)))

(event `Key|E`
  (params (Key :type "Key Structure"))
  (:`Pressed`
    (`self.SetWorldRotationAxis` (0.0 -1.0 0.0))
    (`self.ArrayCleaning`)
    (`self.AssignRotationTargets`)
    (bind (_direction _shakeoffset) (`Timeline|TL_ShakeWorldRotationStarted` :!via `PlayFromStart`)
      (:`Update`
        (`SceneComponent.K2_SetRelativeRotation` (`self.DefaultSceneRoot`) (`KismetMathLibrary.MakeRotator` 0.0 _shakeoffset _shakeoffset) false false))
      (:`Finished`
        (`KismetSystemLibrary.Delay` 0.1)
        (bind (_direction_2 _rotation) (`Timeline|TL_RotateWorld` :!via `PlayFromStart`)
          (:`Update`
            (`self.RotationOfEachComponent` _rotation))
          (:`Finished`
            (bind (_direction_3 _shakeoffset_2) (`Timeline|TL_ShakeWorldRotationEnded` :!via `PlayFromStart`)
              (:`Update`
                (`SceneComponent.K2_SetRelativeRotation` (`self.DefaultSceneRoot`) (`KismetMathLibrary.MakeRotator` 0.0 _shakeoffset_2 _shakeoffset_2) false false)
                (`self.ResetWorldRotationAxis`)))))))))

(fn `AddRotationTarget`
  (params (`TargetComponent ` :type "SceneComponent Object Reference"))
  (`KismetArrayLibrary.Array_Add` (`self.ComponentsToRotate`) `TargetComponent `)
  (bind _output_get (set `self.StartRot` (`SceneComponent.K2_GetComponentRotation` `TargetComponent `)))
  (`KismetArrayLibrary.Array_Add` (`self.StartRotations`) _output_get)
  (bind _output_get_2 (set `self.TargetRot` (`KismetMathLibrary.MakeRotator` (+ (.roll _output_get) 90.0) (.pitch _output_get) (.yaw _output_get))))
  (`KismetArrayLibrary.Array_Add` (`self.TargetRotations`) _output_get_2)
  (for (_array_element _array_index) (`self.ComponentsToRotate`)
    (`KismetSystemLibrary.PrintString` (`KismetStringLibrary.Concat_StrStr` (`KismetStringLibrary.Conv_IntToString` _array_index) ". " (`KismetSystemLibrary.GetDisplayName` _array_element)) true true (struct :`G` 0.66 :`B` 1.0 :`A` 1.0) 10.0)))

(fn `ArrayCleaning`
  (`KismetArrayLibrary.Array_Clear` (`self.ComponentsToRotate`))
  (`KismetArrayLibrary.Array_Clear` (`self.TargetRotations`))
  (`KismetArrayLibrary.Array_Clear` (`self.StartRotations`)))

(fn `AssignRotationTargets`
  (`self.AddRotationTarget` (`self.SkySphere`))
  (bind _asbp_third_person_character (cast `/Game/LOGIC/Blueprints/BP_ThirdPersonCharacter` (`GameplayStatics.GetPlayerCharacter` 0)))
  (bind _hitcomponent (`/Game/LOGIC/Blueprints/BP_ThirdPersonCharacter.GetCurrentBaseCube` _asbp_third_person_character))
  (bind _output_get (set `self.BaseCube` _hitcomponent))
  (for _array_element (`self.AllCubes`)
    (if (!= _array_element _output_get)
      (`self.AddRotationTarget` _array_element))))

(fn `ResetWorldRotationAxis`
  (bind _asbp_third_person_character (cast `/Game/LOGIC/Blueprints/BP_ThirdPersonCharacter` (`GameplayStatics.GetPlayerCharacter` 0)))
  (set `/Game/LOGIC/Blueprints/BP_ThirdPersonCharacter.WorldRotationAxis` (0.0 0.0 0.0) _asbp_third_person_character))

(fn `RotateComponent `
  (params (AngleDelta :type "Float (double-precision)") (TargetComponent :type "SceneComponent Object Reference")))

(fn `RotationOfEachComponent`
  (params (InputPin :type "Float (single-precision)"))
  (for (_array_element _array_index) (`self.ComponentsToRotate`)
    (`SceneComponent.K2_SetWorldRotation` _array_element (`KismetMathLibrary.RLerp` (`|GetArrayItem` (`self.StartRotations`) _array_index) (`|GetArrayItem` (`self.TargetRotations`) _array_index) InputPin) false false)))

(fn `SetWorldRotationAxis`
  (params (WorldRotationAxis :type "Vector Structure"))
  (bind _asbp_third_person_character (cast `/Game/LOGIC/Blueprints/BP_ThirdPersonCharacter` (`GameplayStatics.GetPlayerCharacter` 0)))
  (set `/Game/LOGIC/Blueprints/BP_ThirdPersonCharacter.WorldRotationAxis` WorldRotationAxis _asbp_third_person_character))

(fn `UserConstructionScript`
  (bind _allcubes (`self.AllCubes`))
  (`KismetArrayLibrary.Array_Add` _allcubes (`self.CubeLeft`))
  (`KismetArrayLibrary.Array_Add` _allcubes (`self.CubeRight`))
  (`KismetArrayLibrary.Array_Add` _allcubes (`self.CubeCenter`)))