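; Rounded cube actor that rotates as the player character moves from its flat zone into a curved edge.
; The construction script derives edge width from mesh bounds; Tick converts player position in mesh space into dominant-axis direction and curve depth.
; These set a target atop AccumulatedRotation, whose RInterpTo result is added as world rotation, not set.
; The step-commit check for full depth is nested inside the below-full-depth branch.
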(event `self.ReceiveBeginPlay`
  (`self.UpdatePlayerRef`))

(event `self.ReceiveTick`
  (params (DeltaSeconds :type "Float (single-precision)"))
  (bind _distanceintocurve_ (`self.GetDistanceIntoCurve`))
  (bind (_isatedge _rotationdirection) (`self.GetRotationDirection`))
  (if _isatedge
    (if (< _distanceintocurve_ 1.0)
      (bind _targetrotation (`self.CalculateTargetRotation` _rotationdirection _distanceintocurve_))
      (`self.RotateCube` _targetrotation DeltaSeconds)
      (if (>= _distanceintocurve_ 1.0)
        (if (== (`self.HasUpdatedRotationThisStep`) false)
          (`self.UpdateAccumulatedRotation` _rotationdirection)
          (set `self.HasUpdatedRotationThisStep` true)
          (if (< _distanceintocurve_ 0.9)
            (set `self.HasUpdatedRotationThisStep` false)))))))

(fn `CalculateTargetRotation`
  (params (`RotationDirection ` :type "Vector Structure") (`DistanceIntoCurve ` :type "Float (double-precision)"))
  (returns (TargetRotation :type "Rotator Structure"))
  (bind _accumulatedrotation_ (`self.AccumulatedRotation `))
  (bind _returnvalue (* `DistanceIntoCurve ` (`self.MaxRotationAngle`)))
  (if (`self.HasUpdatedRotationThisStep`)
    (return _accumulatedrotation_)
    (else
      (return (`KismetMathLibrary.ComposeRotators` _accumulatedrotation_ (`KismetMathLibrary.MakeRotator` (* _returnvalue (.x `RotationDirection `)) (* _returnvalue (.y `RotationDirection `))))))))

(fn `GetDistanceIntoCurve`
  (returns (`DistanceIntoCurve ` :type "Float (double-precision)"))
  (bind _returnvalue (- (`self.CubeHalfSize`) (`self.EdgeThreshold`)))
  (bind _output_get (set `self.DeltaX` (`KismetMathLibrary.FMax` 0.0 (- (`KismetMathLibrary.Abs` (.x (`KismetMathLibrary.InverseTransformLocation` (`SceneComponent.K2_GetComponentToWorld` (`self.Mesh`)) (`self.K2_GetActorLocation` (`self.PlayerRef`))))) _returnvalue))))
  (bind _output_get_2 (set `self.DeltaY` (`KismetMathLibrary.FMax` 0.0 (- (`KismetMathLibrary.Abs` (.y (`KismetMathLibrary.InverseTransformLocation` (`SceneComponent.K2_GetComponentToWorld` (`self.Mesh`)) (`self.K2_GetActorLocation` (`self.PlayerRef`))))) _returnvalue))))
  (return (`KismetMathLibrary.FMax` (`KismetMathLibrary.FClamp` (/ _output_get_2 (`self.EdgeThreshold`))) (`KismetMathLibrary.FClamp` (/ _output_get (`self.EdgeThreshold`))))))

(fn `GetRotationDirection`
  (returns (IsAtEdge :type Boolean) (RotationDirection :type "Vector Structure"))
  (bind _returnvalue (- (`self.CubeHalfSize`) (`self.EdgeThreshold`)))
  (bind _x (.x (`KismetMathLibrary.InverseTransformLocation` (`SceneComponent.K2_GetComponentToWorld` (`self.Mesh`)) (`self.K2_GetActorLocation` (`self.PlayerRef`)))))
  (bind _y (.y (`KismetMathLibrary.InverseTransformLocation` (`SceneComponent.K2_GetComponentToWorld` (`self.Mesh`)) (`self.K2_GetActorLocation` (`self.PlayerRef`)))))
  (bind _returnvalue_2 (or (> (`KismetMathLibrary.Abs` _x) _returnvalue) (> (`KismetMathLibrary.Abs` _y) _returnvalue)))
  (if (> (`KismetMathLibrary.Abs` _x) (`KismetMathLibrary.Abs` _y))
    (if (> _x 0.0)
      (return _returnvalue_2 (0.0 1.0 0.0))
      (else
        (return _returnvalue_2 (0.0 -1.0 0.0))))
    (elif (> _y 0.0)
      (return _returnvalue_2 (-1.0 0.0 0.0))
      (else
        (return _returnvalue_2 (1.0 0.0 0.0))))))

(fn `RotateCube`
  (params (`TargetRotation ` :type "Rotator Structure") (DeltaTime :type "Float (double-precision)"))
  (`SceneComponent.K2_AddWorldRotation` (`self.Mesh`) (`KismetMathLibrary.RInterpTo` (`SceneComponent.RelativeRotation` (`self.Mesh`)) `TargetRotation ` DeltaTime (`self.InterpSpeed`)) false false))

(fn `UpdateAccumulatedRotation`
  (params (RotationDirection :type "Vector Structure"))
  (set `self.AccumulatedRotation ` (`KismetMathLibrary.ComposeRotators` (`self.AccumulatedRotation `) (`KismetMathLibrary.MakeRotator` (.x (* RotationDirection (`self.MaxRotationAngle`))) (.y (* RotationDirection (`self.MaxRotationAngle`)))))))

(fn `UpdatePlayerRef`
  (returns (PlayerRef :type "/Game/LOGIC/Blueprints/BP_ThirdPersonCharacter Object Reference"))
  (bind _asbp_third_person_character (cast `/Game/LOGIC/Blueprints/BP_ThirdPersonCharacter` (`GameplayStatics.GetPlayerCharacter` 0)))
  (bind _output_get (set `self.PlayerRef` _asbp_third_person_character))
  (return _output_get))

(fn `UserConstructionScript`
  (bind (_min _max) (break `Box` (`StaticMesh.GetBoundingBox` (`StaticMeshComponent.StaticMesh` (`self.Mesh`)))))
  (`parent.UserConstructionScript`)
  (bind _output_get (set `self.CubeHalfSize` (`KismetMathLibrary.FMax` (.x (/ (- _max _min) 2.0)) (.y (/ (- _max _min) 2.0)))))
  (set `self.EdgeThreshold` (* _output_get (- 1.0 (`self.FlatZoneRatio`)))))