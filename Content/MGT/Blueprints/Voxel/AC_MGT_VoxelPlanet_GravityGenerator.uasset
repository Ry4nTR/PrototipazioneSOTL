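; Actor component that gives a voxel planet gravity by spawning a giant planet gravity actor at its owner.
; On BeginPlay it spawns BP_MGT_GiantPlanet at the owner's location scaled by CoreScale, copies GravityScale onto it and attaches it to the owner.
; It sets the spawned actor's tags to MGT_VoxelGen and the owner's to MGT_VoxelMesh, replacing any existing tags.
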(event `self.ReceiveBeginPlay`
  (bind _corescale (`self.CoreScale`))
  (bind _returnvalue (`|SpawnActorFromClass` "/Game/MGT/Blueprints/DynamicGravityGenerators/GiantGenerators/BP_MGT_GiantPlanet.BP_MGT_GiantPlanet_C" (`KismetMathLibrary.MakeTransform` (`Actor.K2_GetActorLocation` (`self.GetOwner`)) (struct) (`KismetMathLibrary.MakeVector` _corescale _corescale _corescale)) "Undefined" "OverrideRootScale" null "NewEnumerator0" null))
  (set `/Game/MGT/Blueprints/DynamicGravityGenerators/ParentMatrice/BP_MGT_GravityGenerator.GravityScale` (`self.GravityScale`) _returnvalue)
  (`Actor.K2_AttachToActor` _returnvalue (`self.GetOwner`) "None" "KeepWorld" "KeepWorld" "KeepWorld" true)
  (set `Actor.Tags` (`|MakeArray` "MGT_VoxelGen" :!type "Name") _returnvalue)
  (set `Actor.Tags` (`|MakeArray` "MGT_VoxelMesh" :!type "Name") (`self.GetOwner`)))