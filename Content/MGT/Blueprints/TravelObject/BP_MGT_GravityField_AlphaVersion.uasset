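; Alpha MGT gravity field actor that pulls, repels or directionally moves physics objects such as Chaos fragments and ragdolls, not players.
; On BeginPlay, GravityType selects a radial or uniform vector added as a persistent linear-velocity field, overriding other MGT gravity; Ring World only prints unavailable.
; Unless influence is unlimited, a radial falloff culls the field outside the sphere.
; The construction script sizes the spheres and shows DIRECTION only for directional gravity.
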(event `self.ReceiveBeginPlay`
  ;[1 1 1] ALPHA VERSION
  ; This gravity field system will only apply a gravity force on objects (not players)
  ; It can be used to apply a gravity to chaos mesh parts
  ; It can also work for ragdolls
  ; It apply a linear velocity (instead of a force) that's why this system will overide all other MGT's Gravity systems
  (switch `/Game/MGT/Blueprints/TravelObject/Enum_GravityType` (`self.GravityType`)
    (:`NewEnumerator3`
      (`self.DirectionalField`))
    (:`NewEnumerator0`
      (`self.SphericalGravity`))
    (:`NewEnumerator1`
      (`self.RepulsiveGravity`))
    (:`NewEnumerator2`
      (`KismetSystemLibrary.PrintString` "Ring World Gravity Field not available for now" true true (struct :`G` 0.66 :`B` 1.0 :`A` 1.0) 50.0))))

(event `SphericalGravity`
  (bind _returnvalue (`RadialVector.SetRadialVector` (`self.RadialVector`) (* (`self.GravityForce`) -1.0) (`SceneComponent.K2_GetComponentLocation` (`self.Sphere1`))))
  ;[1 1 1] ALPHA VERSION
  ; This gravity field system will only apply a gravity force on objects (not players)
  ; It can be used to apply a gravity to chaos mesh parts
  ; It can also work for ragdolls
  ; It apply a linear velocity (instead of a force) that's why this system will overide all other MGT's Gravity systems
  ;;[1 1 1] Planet gravity field
  (`FieldSystemComponent.AddPersistentField` (`self.FieldSystemComponent`) true "Field_LinearVelocity" null (cast `FieldNodeBase` (`KismetMathLibrary.SelectObject` _returnvalue (`CullingField.SetCullingField` (`self.CullingField`) (`self.MGT_ComputeFallOff`) _returnvalue "Field_Culling_Outside") (`self.UnlimitedInfluence`)) :!pure true)))

(event `RepulsiveGravity`
  (bind _returnvalue (`RadialVector.SetRadialVector` (`self.RadialVector`) (`self.GravityForce`) (`SceneComponent.K2_GetComponentLocation` (`self.Sphere`))))
  ;[1 1 1] ALPHA VERSION
  ; This gravity field system will only apply a gravity force on objects (not players)
  ; It can be used to apply a gravity to chaos mesh parts
  ; It can also work for ragdolls
  ; It apply a linear velocity (instead of a force) that's why this system will overide all other MGT's Gravity systems
  ;;[1 1 1] Planet gravity field
  (`FieldSystemComponent.AddPersistentField` (`self.FieldSystemComponent`) true "Field_LinearVelocity" null (cast `FieldNodeBase` (`KismetMathLibrary.SelectObject` _returnvalue (`CullingField.SetCullingField` (`self.CullingField`) (`self.MGT_ComputeFallOff`) _returnvalue "Field_Culling_Outside") (`self.UnlimitedInfluence`)) :!pure true)))

(event `DirectionalField`
  (bind _returnvalue (`UniformVector.SetUniformVector` (`self.UniformVector`) (`self.GravityForce`) (`KismetMathLibrary.SelectVector` (`self.GravityDirection`) (`self.GetActorForwardVector` self) (`self.OvverrideGravityDirection`))))
  ;[1 1 1] ALPHA VERSION
  ; This gravity field system will only apply a gravity force on objects (not players)
  ; It can be used to apply a gravity to chaos mesh parts
  ; It can also work for ragdolls
  ; It apply a linear velocity (instead of a force) that's why this system will overide all other MGT's Gravity systems
  ;;[1 1 1] Directional Gravity Field - need a gravity force >500 to work better
  (`FieldSystemComponent.AddPersistentField` (`self.FieldSystemComponent`) true "Field_LinearVelocity" null (cast `FieldNodeBase` (`KismetMathLibrary.SelectObject` _returnvalue (`CullingField.SetCullingField` (`self.CullingField`) (`self.MGT_ComputeFallOff`) _returnvalue "Field_Culling_Outside") (`self.UnlimitedInfluence`)) :!pure true))
  (if (not (`self.OvverrideGravityDirection`))
    (set `self.GravityDirection` (`self.GetActorForwardVector` self))))

(fn `MGT_ComputeFallOff`
  (returns (ComputeFallOff :type "RadialFalloff Object Reference"))
  (bind _sphere1 (`self.Sphere1`))
  (return (`RadialFalloff.SetRadialFalloff` (`self.RadialFalloff`) 1.0 0.0 1.0 0.0 (`SphereComponent.SphereRadius` _sphere1) (`SceneComponent.K2_GetComponentLocation` _sphere1) "Field_Falloff_Linear")))

(fn `UserConstructionScript`
  (bind _direction (`self.DIRECTION`))
  (`SphereComponent.SetSphereRadius` (`self.Sphere1`) (`self.RadiusOfInfluence`) true)
  (`SceneComponent.SetRelativeScale3D` (`self.Sphere`) (`KismetMathLibrary.Conv_DoubleToVector` (* (`SphereComponent.SphereRadius` (`self.Sphere1`)) 0.02)))
  (`SceneComponent.SetRelativeScale3D` (`self.Sphere1`) (1.0 1.0 1.0))
  (`self.SetActorScale3D` self (1.0 1.0 1.0))
  (switch `/Game/MGT/Blueprints/TravelObject/Enum_GravityType` (`self.GravityType`)
    (:`NewEnumerator3`
      (`SceneComponent.SetVisibility` _direction true false))
    (:`NewEnumerator0`
      (`SceneComponent.SetVisibility` _direction false false :!label _label))
    (:`NewEnumerator1`
      (goto _label))
    (:`NewEnumerator2`
      (goto _label))))